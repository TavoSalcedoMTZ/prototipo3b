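; BP_GameManager is a central coordinator Blueprint linking the player, the horde system and the UI.
; Init events store references to the player, horde system and UI, and GetPlayer returns the stored player.
; StartHorde and EnemyDefeat forward to the horde system, while FinishHorde ends the horde and then opens the store through the UI.
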(event EventInitPlayer
  (params (player :type BP%20First%20Person%20Character%20Object%20Reference))
  (Variables|Default|SetPlayer player))

(event EventInitHordes
  (params (reference :type Hordes%20System%20Object%20Reference))
  (Variables|Default|SetHordesSystem reference))

(event EventStartHorde
  (Default|SpawnHorde (Variables|Default|GetHordesSystem)))

(event EventFinishHorde
  (Default|FinishHorde (Variables|Default|GetHordesSystem))
  (Default|OpenStore (Variables|Default|GetUI)))

(event EventEnemyDefeat
  (Default|EnemyDefeat (Variables|Default|GetHordesSystem)))

(event EventInitWB
  (params (NewParam :type WB%20UI%20Object%20Reference))
  (Variables|Default|SetUI NewParam))

(fn GetPlayer
  (return (Variables|Default|GetPlayer)))