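; Zombie enemy character that takes damage when shot and reports player proximity to its AI.
; Each BeginShoot event prints a debug string and subtracts a fixed, clamped amount of HP; at zero it notifies the GameInstance of the defeat and destroys itself.
; Sphere begin and end overlaps with Player-tagged actors set or clear the IsNear Blackboard bool through two helper functions.
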(event OnComponentBeginOverlap(Sphere)
  (params (OverlappedComponent :type Primitive%20Component%20Object%20Reference) (OtherActor :type Actor%20Object%20Reference) (OtherComp :type Primitive%20Component%20Object%20Reference) (OtherBodyIndex :type Integer) (bFromSweep :type Boolean) (SweepResult :type Hit%20Result%20Structure%20%28by%20ref%29))
  (CallFunction|EncenderAcermiento OtherActor))

(event OnComponentEndOverlap(Sphere)
  (params (OverlappedComponent :type Primitive%20Component%20Object%20Reference) (OtherActor :type Actor%20Object%20Reference) (OtherComp :type Primitive%20Component%20Object%20Reference) (OtherBodyIndex :type Integer))
  (CallFunction|ApagarAcercamiento OtherActor))

(event EventBeginPlay)

(event Collision|EventActorBeginOverlap
  (params (OtherActor :type Actor%20Object%20Reference)))

(event EventTick
  (params (DeltaSeconds :type Float%20%28single-precision%29)))

(event EventBeginShoot
  (Development|PrintString "Hello")
  (if (> (Variables|Default|GetHP) 0.0)
    (bind _output_get (Variables|Default|SetHP (Math|Float|Clamp(Float) (- (Variables|Default|GetHP) 1e+01) 0.0 5e+02)))
    (if (<= _output_get 0.0)
      (Class|BPIGM|EnemyDefeat(Message) (Game|GetGameInstance))
      (Actor|DestroyActor))))

(fn ConstructionScript)

(fn ApagarAcercamiento
  (params (self2 :type Actor%20Object%20Reference))
  (if (Actor|ActorHasTag self2 "Player")
    (AI|Components|Blackboard|SetValueasBool (AI|GetBlackboard 0) (Utilities|Name|MakeLiteralName "IsNear") false)))

(fn EncenderAcermiento
  (params (self2 :type Actor%20Object%20Reference))
  (if (Actor|ActorHasTag self2 "Player")
    (AI|Components|Blackboard|SetValueasBool (AI|GetBlackboard 0) (Utilities|Name|MakeLiteralName "IsNear") true)))